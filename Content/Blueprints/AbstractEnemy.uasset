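; Base enemy actor that damages the player character on hurtbox overlap and shows a health bar widget while the player is within a radius.
; Incoming damage is reduced by a resistance matched to its damage type (capped at 95%, immune at extreme values) and a diminishing-returns DEF modifier.
; A DoOnce gate ignores further hits for a second after each non-lethal one.
; On death it ragdolls, then spawns a gold coin and destroys itself.
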(event `self.ReceiveBeginPlay`
  (bind _asenemy_data_widget (cast `/Game/Blueprints/EnemyDataWidget` (`WidgetComponent.GetUserWidgetObject` (`self.HealthBar`))))
  (bind _output_get (set `self.As Enemy Data Widget` _asenemy_data_widget))
  (set `/Game/Blueprints/EnemyDataWidget.MaxHealth` (`self.MaxHP`) _output_get)
  (set `/Game/Blueprints/EnemyDataWidget.CurrentHealth` (`self.CurrentHP`) _output_get))

(event `self.HurtBox.OnComponentBeginOverlap`
  (params (OverlappedComponent :type "PrimitiveComponent Object Reference") (OtherActor :type "Actor Object Reference") (OtherComp :type "PrimitiveComponent Object Reference") (OtherBodyIndex :type Integer) (bFromSweep :type Boolean) (SweepResult :type "HitResult Structure (by ref)"))
  (bind _asbp_third_person_character (cast `/Game/ThirdPerson/Blueprints/BP_ThirdPersonCharacter` OtherActor))
  (`GameplayStatics.ApplyDamage` _asbp_third_person_character (`self.ATK`) null null (`self.Damage Type Class`)))

(event `self.ReceiveTick`
  (params (DeltaSeconds :type "Float (single-precision)")))

(event `self.ReceiveAnyDamage`
  (params (Damage :type "Float (single-precision)") (DamageType :type "DamageType Object Reference") (InstigatedBy :type "Controller Object Reference") (DamageCauser :type "Actor Object Reference"))
  (bind _as_enemy_data_widget (`self.As Enemy Data Widget`))
  (`/Engine/EditorBlueprintResources/StandardMacros.DoOnce` false :!label _label
    (:`Completed`
      (bind _damagedealt (`self.CalculateDamage` Damage DamageType))
      (bind _output_get (set `self.CurrentHP` (- (`self.CurrentHP`) _damagedealt)))
      (if (<= _output_get 0.0)
        (`KismetSystemLibrary.PrintText` "Target would die")
        (set `/Game/Blueprints/EnemyDataWidget.CurrentHealth` 0.0 _as_enemy_data_widget)
        (`PrimitiveComponent.SetSimulatePhysics` (`self.SkeletalMesh`) true)
        (`KismetSystemLibrary.Delay` 1.5)
        (bind _returnvalue (`|SpawnActorFromClass` "/Game/Blueprints/Coin.Coin_C" (`self.GetTransform`) "Undefined" "OverrideRootScale" null null))
        (set `/Game/Blueprints/Coin.Value` (`self.DroppedGold`) _returnvalue)
        (`self.K2_DestroyActor`)
        (else
          (set `/Game/Blueprints/EnemyDataWidget.CurrentHealth` _output_get _as_enemy_data_widget)
          (`KismetSystemLibrary.PrintString` (`KismetStringLibrary.Conv_DoubleToString` _damagedealt))
          (`KismetSystemLibrary.Delay` 1.0)
          (goto _label :!via `Reset`))))))

(event `self.HealthBarDrawRadius.OnComponentBeginOverlap`
  (params (OverlappedComponent :type "PrimitiveComponent Object Reference") (OtherActor :type "Actor Object Reference") (OtherComp :type "PrimitiveComponent Object Reference") (OtherBodyIndex :type Integer) (bFromSweep :type Boolean) (SweepResult :type "HitResult Structure (by ref)"))
  (cast `/Game/ThirdPerson/Blueprints/BP_ThirdPersonCharacter` OtherActor)
  (`SceneComponent.SetVisibility` (`self.HealthBar`) true false))

(event `self.HealthBarDrawRadius.OnComponentEndOverlap`
  (params (OverlappedComponent :type "PrimitiveComponent Object Reference") (OtherActor :type "Actor Object Reference") (OtherComp :type "PrimitiveComponent Object Reference") (OtherBodyIndex :type Integer))
  (cast `/Game/ThirdPerson/Blueprints/BP_ThirdPersonCharacter` OtherActor)
  (`SceneComponent.SetVisibility` (`self.HealthBar`) false false))

(fn `CalculateDamage`
  (params (DamageTaken :type "Float (double-precision)") (DamageType :type "DamageType Object Reference"))
  (returns (DamageDealt :type "Float (double-precision)"))
  (bind _res (`self.GetCorrespondingRES` DamageType))
  (bind _defmodifier (`self.GetDEFModifier`))
  (if (> _res 500.0)
    (return 0.0)
    (elif (> _res 0.95)
      (return (* (* DamageTaken 0.05) _defmodifier))
      (else
        (return (* (* DamageTaken (- 1.0 _res)) _defmodifier))))))

(fn `GetCorrespondingRES`
  (params (DamageTypeTaken :type "DamageType Object Reference"))
  (returns (RES :type "Float (double-precision)"))
  (cast `/Game/Blueprints/DamageType_Physical` DamageTypeTaken
    (:`then`
      (return (`self.PhysicalRES`)))
    (:`CastFailed`
      (cast `/Game/Blueprints/DamageType_Magic` DamageTypeTaken
        (:`then`
          (return (`self.MagicRES`)))
        (:`CastFailed`
          (cast `/Game/Blueprints/DamageType_Water` DamageTypeTaken
            (:`then`
              (return (`self.WaterRES`)))
            (:`CastFailed`
              (cast `/Game/Blueprints/DamageType_Earth` DamageTypeTaken
                (:`then`
                  (return (`self.EarthRES`)))
                (:`CastFailed`
                  (cast `/Game/Blueprints/DamageType_Fire` DamageTypeTaken
                    (:`then`
                      (return (`self.FireRES`)))
                    (:`CastFailed`
                      (cast `/Game/Blueprints/DamageType_Air` DamageTypeTaken
                        (:`then`
                          (return (`self.AirRES`)))
                        (:`CastFailed`
                          (cast `/Game/Blueprints/DamageType_Nature` DamageTypeTaken
                            (:`then`
                              (return (`self.NatureRES`)))
                            (:`CastFailed`
                              (cast `/Game/Blueprints/DamageType_Electric` DamageTypeTaken
                                (:`then`
                                  (return (`self.ElectricRES`)))
                                (:`CastFailed`
                                  (return 0.0))))))))))))))))))

(fn `GetDEFModifier`
  (returns (DEFModifier :type "Float (double-precision)"))
  (return (- 1.0 (/ (`self.DEF`) (+ (`self.DEF`) 100)))))

(fn `OnDeath`)

(fn `UserConstructionScript`)