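; BasicSkill2 is a short-lived skill actor that knocks back enemies it touches.
; On overlap with an AbstractEnemy, it turns on skeletal mesh physics and applies a strong impulse directed away from the skill's location, sending the enemy ragdolling.
; The actor destroys itself half a second after spawning.
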(event `self.ReceiveBeginPlay`
  (`KismetSystemLibrary.Delay` 0.5)
  (`self.K2_DestroyActor`))

(event `self.ReceiveActorBeginOverlap`
  (params (OtherActor :type "Actor Object Reference"))
  (bind _asabstract_enemy (cast `/Game/Blueprints/AbstractEnemy` OtherActor))
  (bind _skeletalmesh (`/Game/Blueprints/AbstractEnemy.SkeletalMesh` _asabstract_enemy))
  (`PrimitiveComponent.SetSimulatePhysics` _skeletalmesh true)
  (`PrimitiveComponent.AddImpulse` _skeletalmesh (* (`KismetMathLibrary.GetDirectionUnitVector` (`self.K2_GetActorLocation`) (`self.K2_GetActorLocation` _asabstract_enemy)) 50000.0) "None" false))

(fn `UserConstructionScript`
  (`parent.UserConstructionScript`))