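; AbstractItem is a base shop pickup that the third-person character buys by walking into it.
; Collision overlap checks the character's HeldGold against ShopCost, then calls the empty OnPickup hook for item effects, deducts the gold and destroys the item.
; A constantly spinning text display shows the price, and a separate InfoDrawRadius overlap toggles a tooltip widget filled from TooltipText.
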(event `self.ReceiveBeginPlay`
  (`TextRenderComponent.K2_SetText` (`self.CostDisplay`) (`KismetTextLibrary.Conv_IntToText` (`self.ShopCost`)))
  (bind _asitem_data_widget (cast `/Game/Blueprints/ItemDataWidget` (`WidgetComponent.GetUserWidgetObject` (`self.Info`))))
  (bind _output_get (set `self.As Item Data Widget` _asitem_data_widget))
  (set `/Game/Blueprints/ItemDataWidget.DisplayInfo` (`self.TooltipText`) _output_get))

(event `self.Collision.OnComponentBeginOverlap`
  (params (OverlappedComponent :type "PrimitiveComponent Object Reference") (OtherActor :type "Actor Object Reference") (OtherComp :type "PrimitiveComponent Object Reference") (OtherBodyIndex :type Integer) (bFromSweep :type Boolean) (SweepResult :type "HitResult Structure (by ref)"))
  (bind _shopcost (`self.ShopCost`))
  (bind _asbp_third_person_character (cast `/Game/ThirdPerson/Blueprints/BP_ThirdPersonCharacter` OtherActor))
  (bind _heldgold (`/Game/ThirdPerson/Blueprints/BP_ThirdPersonCharacter.HeldGold` _asbp_third_person_character))
  (if (>= _heldgold _shopcost)
    (`self.OnPickup`) ; Trigger this item's on pickup effects
    (set `/Game/ThirdPerson/Blueprints/BP_ThirdPersonCharacter.HeldGold` (- _heldgold _shopcost) _asbp_third_person_character) ; Deduct from the character's gold count
    (`self.K2_DestroyActor`) ; And destory the item in the world
    (`KismetSystemLibrary.PrintString` "Item purchased")
    (else
      (`KismetSystemLibrary.PrintString` "Not enough gold"))))

(event `self.ReceiveTick`
  (params (DeltaSeconds :type "Float (single-precision)"))
  (`SceneComponent.K2_AddLocalRotation` (`self.CostDisplay`) (`KismetMathLibrary.MakeRotator` 0.0 0.0 (* DeltaSeconds (`self.DisplayRotationSpeed`))) false false))

(event `self.InfoDrawRadius.OnComponentBeginOverlap`
  (params (OverlappedComponent :type "PrimitiveComponent Object Reference") (OtherActor :type "Actor Object Reference") (OtherComp :type "PrimitiveComponent Object Reference") (OtherBodyIndex :type Integer) (bFromSweep :type Boolean) (SweepResult :type "HitResult Structure (by ref)"))
  (cast `/Game/ThirdPerson/Blueprints/BP_ThirdPersonCharacter` OtherActor)
  (`SceneComponent.SetVisibility` (`self.Info`) true false))

(event `self.InfoDrawRadius.OnComponentEndOverlap`
  (params (OverlappedComponent :type "PrimitiveComponent Object Reference") (OtherActor :type "Actor Object Reference") (OtherComp :type "PrimitiveComponent Object Reference") (OtherBodyIndex :type Integer))
  (cast `/Game/ThirdPerson/Blueprints/BP_ThirdPersonCharacter` OtherActor)
  (`SceneComponent.SetVisibility` (`self.Info`) false false))

(fn `OnPickup`)

(fn `UserConstructionScript`)